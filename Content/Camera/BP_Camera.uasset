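; Camera pawn that orbits by click-dragging with a visible mouse cursor and zooms with the mouse wheel.
; Click opens a gate on Tick that feeds per-frame cursor movement, scaled by Sensitivity, into controller yaw and pitch; release closes it.
; A second, drag-offset rotation branch depends on a Pressed flag that this graph never sets true.
; The wheel adjusts spring arm length within a clamped range.
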(event Custom|Rotate%20Camera
  (bind _returnvalue (Game|GetPlayerController 0))
  (bind _sensitivity (Variables|Default|GetSensitivity))
  (bind (_locationx _locationy) (Game|Player|GetMousePosition _returnvalue))
  (bind _returnvalue_2 (Math|Vector2D|MakeVector2D _locationx _locationy))
  ;[1 1 1] Camera controlls
  (bind _output_get (Variables|Default|SetStartVector _returnvalue_2))
  (Variables|Default|SetEndVector _output_get)
  (Utilities|FlowControl|Gate true) ; enters at Open
)

(event Custom|ChangeCamPosition
  (params (Pressed :type Boolean))
  (bind _returnvalue (Game|GetPlayerController 0))
  (bind _sensitivity (Variables|Default|GetSensitivity))
  (bind (_locationx _locationy) (Game|Player|GetMousePosition _returnvalue))
  (bind _returnvalue_2 (Math|Vector2D|MakeVector2D _locationx _locationy))
  ;[1 1 1] Camera controlls
  (if Pressed
    (CallFunction|RotateCamera)
    (else
      (Variables|Default|SetPressed false)
      (Utilities|FlowControl|Gate true) ; enters at Close
    )))

(event EventBeginPlay
  (Variables|/Script/Engine.PlayerController|SetbShowMouseCursor (Game|GetPlayerController 0) true))

(event EventTick
  (params (DeltaSeconds :type Float%20%28single-precision%29))
  (bind _returnvalue (Game|GetPlayerController 0))
  (bind _returnvalue_2 (Utilities|Time|GetWorldDeltaSeconds))
  (bind _returnvalue_3 (Game|GetPlayerController 0))
  (bind _sensitivity (Variables|Default|GetSensitivity))
  (bind _sensitivity_2 (Variables|Default|GetSensitivity))
  (bind (_locationx _locationy) (Game|Player|GetMousePosition _returnvalue_3))
  (bind (_locationx_2 _locationy_2) (Game|Player|GetMousePosition _returnvalue))
  (bind _returnvalue_4 (Math|Vector2D|MakeVector2D _locationx_2 _locationy_2))
  (bind _returnvalue_5 (Math|Vector2D|MakeVector2D _locationx _locationy))
  ;[1 1 1] Camera controlls
  (Utilities|FlowControl|Sequence
    (:then_0
      (if (Variables|Default|GetPressed)
        (if (> (Math|Float|Absolute(Float) (Math|Vector2D|Vector2DLength (- (Variables|Default|GetStartVector) _returnvalue_5))) 0.0)
          (Variables|Default|SetEndVector _returnvalue_5)
          (Pawn|Input|AddControllerYawInput (* (* (.X (Math|Vector2D|BreakVector2D (- (Variables|Default|GetStartVector) (Variables|Default|GetEndVector)))) _returnvalue_2 _sensitivity) -1.0))
          (Pawn|Input|AddControllerPitchInput (* (* (.Y (Math|Vector2D|BreakVector2D (- (Variables|Default|GetStartVector) (Variables|Default|GetEndVector)))) _returnvalue_2 _sensitivity) -1.0)))))
    (:then_1
      (Utilities|FlowControl|Gate true
        (:Exit
          (Variables|Default|SetStartVector "(X=10000000.000000,Y=10000000.000000)")
          (Pawn|Input|AddControllerYawInput (.x (* (- _returnvalue_4 (Variables|Default|GetEndVector)) (* _sensitivity_2 (/ _sensitivity_2 4.0)))))
          (Pawn|Input|AddControllerPitchInput (.y (* (- _returnvalue_4 (Variables|Default|GetEndVector)) (* _sensitivity_2 (/ _sensitivity_2 4.0)))))
          (Variables|Default|SetEndVector _returnvalue_4))))))

(event Input|ActionEvents|InputActionClick
  (params (Key :type Key%20Structure :default "None"))
  ;[1 1 1] Camera controlls
  (:Pressed
    (CallFunction|ChangeCamPosition true))
  (:Released
    (CallFunction|ChangeCamPosition false)))

(event Input|MouseEvents|MouseWheelAxis
  (params (AxisValue :type Float%20%28single-precision%29))
  ;[1 1 1] Camera controlls
  (CallFunction|ChangeSpringArmLength (* AxisValue -1.0)))

(fn ConstructionScript)

(fn ChangeSpringArmLength
  (params (Axis :type Float%20%28single-precision%29))
  (bind _springarm (Variables|Default|GetSpringArm))
  (Variables|/Script/Engine.SpringArmComponent|SetTargetArmLength _springarm (Math|Float|Min(Float) (Math|Float|Max(Float) (+ (* Axis (LocalVariables|GetSensitivy)) (Variables|/Script/Engine.SpringArmComponent|GetTargetArmLength _springarm)) 5e+02) 3e+03)))