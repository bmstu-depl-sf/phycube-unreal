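; BP_ParticalBase is a particle actor base that can leave a trail of BP_Trail actors as it moves.
; InitTrails starts a looping timer when trails are enabled, and SpawnTrail spawns a segment at the last recorded position, passing the current location as its SourcePoint.
; Each segment is stored in an array, which ClearTrails destroys after stopping the timer.
; BeginPlay only prints a debug string.
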(event Custom|SpawnTrail
  (bind _returnvalue (Transformation|GetActorLocation))
  (bind _returnvalue_2 (Game|SpawnActorfromClass "/Game/Effects/BP_Trail.BP_Trail_C" (Math|Transform|MakeTransform (Variables|Default|GetCurrentPosition) "0, 0, 0" "1,1,1") "Undefined" 0 _returnvalue 0))
  (Variables|Default|SetCurrentPosition _returnvalue)
  (Utilities|Array|Add (Variables|Default|GetTrails) _returnvalue_2))

(event Custom|InitTrails
  (if (Variables|BPParticalBase|GetIsTrailOn)
    (bind _returnvalue (Utilities|Time|SetTimerbyEvent (delegate Custom|SpawnTrail) (Variables|BPParticalBase|GetTimer) true))
    (Variables|Default|SetTrailTimerHandle _returnvalue)
    (Variables|Default|SetCurrentPosition (Transformation|GetActorLocation))))

(event Custom|ClearTrails
  (if (Variables|BPParticalBase|GetIsTrailOn)
    (Utilities|Time|ClearandInvalidateTimerbyHandle (Variables|Default|GetTrailTimerHandle))
    (for _array_element (Variables|Default|GetTrails)
      (Actor|DestroyActor _array_element))))

(event EventBeginPlay
  (Development|PrintString "Hello"))

(event EventDestroyed)

(fn ConstructionScript)