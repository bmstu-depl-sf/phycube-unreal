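; BP_CameraController is a player controller that manages the menu widgets for particles, forces and graphics settings.
; On BeginPlay it creates all five widgets, passes the BP_OprimizedGameModeBase reference to the three settings panels, and shows the main menu.
; CloseMenu swaps the main menu and panels for the GetMenu widget, and OpenMenu restores the main menu.
; RemoveFromParantWidgets hides just the three panels.
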(event EventBeginPlay
  (bind _asbp_oprimized_game_mode_base (Utilities|Casting|CastToBP_OprimizedGameModeBase (Game|GetGameMode)))
  (bind _returnvalue (UserInterface|CreateWidget "/Game/Menu/WBP_GetMenu.WBP_GetMenu_C" self))
  (Variables|Default|SetGetMenu _returnvalue)
  (bind _returnvalue_2 (UserInterface|CreateWidget "/Game/Menu/WBP_Particals.WBP_Particals_C" self))
  (bind _output_get (Variables|Default|SetParticalsMenu _returnvalue_2))
  (Variables|/Game/Menu/WBP_Particals.WBP_Particals_C|SetGameMode _output_get _asbp_oprimized_game_mode_base)
  (bind _returnvalue_3 (UserInterface|CreateWidget "/Game/Menu/WBP_Forces.WBP_Forces_C" self))
  (bind _output_get_2 (Variables|Default|SetForcesMenu _returnvalue_3))
  (Variables|/Game/Menu/WBP_Forces.WBP_Forces_C|SetGameMode _output_get_2 _asbp_oprimized_game_mode_base)
  (bind _returnvalue_4 (UserInterface|CreateWidget "/Game/Menu/WBP_Graphic.WBP_Graphic_C" self))
  (bind _output_get_3 (Variables|Default|SetGraphicMenu _returnvalue_4))
  (Variables|/Game/Menu/WBP_Graphic.WBP_Graphic_C|SetGameMode _output_get_3 _asbp_oprimized_game_mode_base)
  (bind _returnvalue_5 (UserInterface|CreateWidget "/Game/Menu/WBP_Menu.WBP_Menu_C" self))
  (bind _output_get_4 (Variables|Default|SetMenu _returnvalue_5))
  (UserInterface|Viewport|AddtoViewport _output_get_4 0))

(fn ConstructionScript)

(fn RemovefromParantWidgets
  (Widget|RemovefromParent (Variables|Default|GetParticalsMenu))
  (Widget|RemovefromParent (Variables|Default|GetForcesMenu))
  (Widget|RemovefromParent (Variables|Default|GetGraphicMenu)))

(fn CloseMenu
  (Widget|RemovefromParent (Variables|Default|GetParticalsMenu))
  (Widget|RemovefromParent (Variables|Default|GetForcesMenu))
  (Widget|RemovefromParent (Variables|Default|GetGraphicMenu))
  (Widget|RemovefromParent (Variables|Default|GetMenu))
  (UserInterface|Viewport|AddtoViewport (Variables|Default|GetGetMenu) 0))

(fn OpenMenu
  (Widget|RemovefromParent (Variables|Default|GetGetMenu))
  (UserInterface|Viewport|AddtoViewport (Variables|Default|GetMenu) 0))