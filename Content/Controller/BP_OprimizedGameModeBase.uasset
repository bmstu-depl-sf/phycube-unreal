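; Game mode for a charged-particle simulation in electric and magnetic fields, acting as the central control for spawning, field settings, pause and visibility.
; It spawns electrons, protons or JSON-defined custom particles at the spawner when unpaused and unblocked, singly or on looping timers.
; Field setters convert angles and magnitude into vectors, rotate the arrow actors and push values to all live particles.
; Helpers toggle grid, axes and force arrows or destroy all particles.
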(event Custom|SpawnElectron
  ;[1 1 1] Spawn Electron
  (if (not (Variables|Default|GetIsPaused))
    (bind _outactors (Actor|GetAllActorsOfClass "/Game/Particals/BP_ParticalSpawner.BP_ParticalSpawner_C"))
    (if (not (Variables|/Game/Particals/BP_ParticalSpawner.BP_ParticalSpawner_C|GetIsOverlap (Utilities|Array|Get(acopy) _outactors)))
      (bind _returnvalue (Game|SpawnActorfromClass "/Game/Particals/BP_ParticalElectron.BP_ParticalElectron_C" (Transformation|GetActorTransform (Utilities|Array|Get(acopy) _outactors)) "Undefined" 0 0))
      (Utilities|IsValid _returnvalue
        (:Is%20Valid
          (Class|ParticalBase|UpdateInitImpulse _returnvalue (Variables|Default|GetInitImpulse))
          (Class|ParticalBase|UpdateElectricForce _returnvalue (Variables|Default|GetElectricStrength))
          (Variables|/Script/SELF.ParticalBase|SetMagneticInduction _returnvalue (Variables|Default|GetMagneticInduction))
          (Variables|/Script/SELF.ParticalBase|SetIsTrailOn _returnvalue (Variables|Default|GetIsTrailOn)))))))

(event Custom|Update%20Data
  (bind _path (Variables|Default|GetPath))
  (bind _particaljson (Variables|Default|GetParticalJson))
  (Class|ParticalJsonComponent|LoadJson _particaljson _path)
  (Variables|Default|SetParticle%20Data (Variables|/Script/SELF.ParticalJsonComponent|GetParticleData _particaljson))
  (Development|PrintString _path))

(event Custom|SpawnProton
  ;[1 1 1] Spawn Proton
  (if (not (Variables|Default|GetIsPaused))
    (bind _outactors (Actor|GetAllActorsOfClass "/Game/Particals/BP_ParticalSpawner.BP_ParticalSpawner_C"))
    (if (not (Variables|/Game/Particals/BP_ParticalSpawner.BP_ParticalSpawner_C|GetIsOverlap (Utilities|Array|Get(acopy) _outactors)))
      (bind _returnvalue (Game|SpawnActorfromClass "/Game/Particals/BP_ParticalProton.BP_ParticalProton_C" (Transformation|GetActorTransform (Utilities|Array|Get(acopy) _outactors)) "Undefined" 0 0))
      (Utilities|IsValid _returnvalue
        (:Is%20Valid
          (Class|ParticalBase|UpdateInitImpulse _returnvalue (Variables|Default|GetInitImpulse))
          (Class|ParticalBase|UpdateElectricForce _returnvalue (Variables|Default|GetElectricStrength))
          (Variables|/Script/SELF.ParticalBase|SetMagneticInduction _returnvalue (Variables|Default|GetMagneticInduction))
          (Variables|/Script/SELF.ParticalBase|SetIsTrailOn _returnvalue (Variables|Default|GetIsTrailOn)))))))

(event Custom|SpawnCustomParticle
  (bind _id (Variables|Default|GetId))
  (bind _particle_data (Variables|Default|GetParticle%20Data))
  (bind _returnvalue (Utilities|Array|Length _particle_data))
  (bind _returnvalue_2 (Math|Integer|Min(Integer) _id _returnvalue))
  (bind _output (Utilities|Array|Get(acopy) _particle_data _returnvalue_2))
  (bind (_name _trail _impulse _mass _charge _timer _rate _red _green _blue) (Utilities|Struct|BreakParticleDataStruct _output))
  ;[1 1 1] Custom partical spawn
  (if (not (Variables|Default|GetIsPaused))
    (bind _outactors (Actor|GetAllActorsOfClass "/Game/Particals/BP_ParticalSpawner.BP_ParticalSpawner_C"))
    (if (not (Variables|/Game/Particals/BP_ParticalSpawner.BP_ParticalSpawner_C|GetIsOverlap (Utilities|Array|Get(acopy) _outactors)))
      (bind _returnvalue_3 (Game|SpawnActorfromClass "/Game/Particals/BP_ParticalCustom.BP_ParticalCustom_C" (Transformation|GetActorTransform (Utilities|Array|Get(acopy) _outactors)) "Undefined" 0 0))
      (Utilities|IsValid _returnvalue_3
        (:Is%20Valid
          (Class|ParticalBase|SetUp _returnvalue_3 _trail _impulse _mass _charge _timer)
          (Class|ParticalBase|UpdateInitImpulse _returnvalue_3 (Variables|Default|GetInitImpulse))
          (Class|ParticalBase|UpdateElectricForce _returnvalue_3 (Variables|Default|GetElectricStrength))
          (Variables|/Script/SELF.ParticalBase|SetMagneticInduction _returnvalue_3 (Variables|Default|GetMagneticInduction))
          (Variables|/Script/SELF.ParticalBase|SetIsTrailOn _returnvalue_3 true)
          (Default|UpdateColor _returnvalue_3 (Math|Color|MakeColor _red _green _blue)))
        (:Is%20Not%20Valid
          (Development|PrintString "Hello"))))))

(event EventBeginPlay
  (bind _path (Variables|Default|GetPath))
  (bind _particaljson (Variables|Default|GetParticalJson))
  (Utilities|FlowControl|Sequence
    (:then_0
      (Class|OptimizedGameModeBase|UnlitModeon)
      ;[1 1 1] Initial visibility
      (CallFunction|SetGridVisibility true)
      (CallFunction|SetAxesVisibility true)
      (CallFunction|SetForcesVisibility true)
      (CallFunction|SetGridVisibility false)
      (CallFunction|SetAxesVisibility false)
      (CallFunction|SetForcesVisibility false))
    (:then_1
      (Class|ParticalJsonComponent|LoadJson _particaljson _path)
      (Variables|Default|SetParticle%20Data (Variables|/Script/SELF.ParticalJsonComponent|GetParticleData _particaljson))
      (Development|PrintString _path))))

(fn ConstructionScript)

(fn DestroyAllParticals
  (bind _outactors (Actor|GetAllActorsOfClass "/Script/SELF.ParticalBase"))
  (for _array_element _outactors
    (Utilities|IsValid _array_element
      (:Is%20Valid
        (Actor|DestroyActor _array_element)))))

(fn SetGridVisibility
  (params (IsHidden :type Boolean))
  (bind _outactors (Actor|GetAllActorsOfClass "/Game/Environment/BP_Grid.BP_Grid_C"))
  (if IsHidden
    (for _array_element _outactors
      (Rendering|SetActorHiddenInGame _array_element false))
    (else
      (for _array_element_2 _outactors
        (Rendering|SetActorHiddenInGame _array_element_2 true)))))

(fn SetAxesVisibility
  (params (IsHidden :type Boolean))
  (bind _outactors (Actor|GetAllActorsOfClass "/Game/Environment/BP_Axis.BP_Axis_C"))
  (if IsHidden
    (for _index (range 0 2)
      (Rendering|SetActorHiddenInGame (Utilities|Array|Get(acopy) _outactors _index) false))
    (else
      (for _index_2 (range 0 2)
        (Rendering|SetActorHiddenInGame (Utilities|Array|Get(acopy) _outactors _index_2) true)))))

(fn SetForcesVisibility
  (params (IsHidden :type Boolean))
  (Utilities|FlowControl|Sequence
    (:then_0
      (bind _outactors (Actor|GetAllActorsOfClass "/Game/Environment/BP_strengthVector.BP_StrengthVector_C"))
      (if IsHidden
        (Rendering|SetActorHiddenInGame (Utilities|Array|Get(acopy) _outactors) false)
        (else
          (Rendering|SetActorHiddenInGame (Utilities|Array|Get(acopy) _outactors) true))))
    (:then_1
      (bind _outactors_2 (Actor|GetAllActorsOfClass "/Game/Environment/BP_MagneticInductionVector.BP_MagneticInductionVector_C"))
      (if IsHidden
        (Rendering|SetActorHiddenInGame (Utilities|Array|Get(acopy) _outactors_2) false)
        (else
          (Rendering|SetActorHiddenInGame (Utilities|Array|Get(acopy) _outactors_2) true))))))

(fn SetForcesRotation
  (params (Alpha :type Float%20%28single-precision%29) (Beta :type Float%20%28single-precision%29) (ElectricForce :type Float%20%28single-precision%29))
  (bind _outactors (Actor|GetAllActorsOfClass "/Game/Environment/BP_strengthVector.BP_StrengthVector_C"))
  (Transformation|SetActorRotation (Utilities|Array|Get(acopy) _outactors) (Math|Rotator|MakeRotator 0.0 Alpha Beta))
  (bind _outactors_2 (Actor|GetAllActorsOfClass "/Game/Environment/BP_StrengthVector_WBP.BP_StrengthVector_WBP_C"))
  (Transformation|SetActorRotation (Utilities|Array|Get(acopy) _outactors_2) (Math|Rotator|MakeRotator 0.0 Alpha Beta))
  (Variables|Default|SetElectircForceScalar ElectricForce)
  (bind _returnvalue (Class|CustomVectorLibrary|RadialtoVector Alpha Beta ElectricForce))
  (Variables|Default|SetElectricStrength _returnvalue)
  (bind _outactors_3 (Actor|GetAllActorsOfClass "/Script/SELF.ParticalBase"))
  (for _array_element _outactors_3
    (Utilities|IsValid _array_element
      (:Is%20Valid
        (Class|ParticalBase|UpdateElectricForce _array_element (Variables|Default|GetElectricStrength))))))

(fn GetForcesRotation
  (bind _strengthrotation (Variables|Default|GetStrengthRotation))
  (return (.pitch _strengthrotation) (.yaw _strengthrotation) (Variables|Default|GetElectircForceScalar)))

(fn LoopSpawnElectron
  (params (IsLoop :type Boolean) (ElectronTimer :type Float%20%28single-precision%29))
  (bind _output_get (Variables|Default|SetIsElectronLoop IsLoop))
  (if _output_get
    (Variables|Default|SetElectronTimer ElectronTimer)
    (bind _returnvalue (Utilities|Time|SetTimerbyEvent (EventDispatchers|CreateEvent :!event Custom|SpawnElectron) (Variables|Default|GetElectronTimer) true))
    (Variables|Default|SetElectronTimerHandle _returnvalue)
    (else
      (Utilities|Time|ClearandInvalidateTimerbyHandle (Variables|Default|GetElectronTimerHandle)))))

(fn LoopSpawnProton
  (params (IsLoop :type Boolean) (ProtonTimer :type Float%20%28single-precision%29))
  (bind _output_get (Variables|Default|SetIsElectronLoop IsLoop))
  (if _output_get
    (Variables|Default|SetProtonTimer ProtonTimer)
    (bind _returnvalue (Utilities|Time|SetTimerbyEvent (EventDispatchers|CreateEvent :!event Custom|SpawnProton) (Variables|Default|GetProtonTimer) true))
    (Variables|Default|SetProtonTimerHandle _returnvalue)
    (else
      (Utilities|Time|ClearandInvalidateTimerbyHandle (Variables|Default|GetProtonTimerHandle)))))

(fn GetInductionsRotation
  (bind _magneticinductionrotation (Variables|Default|GetMagneticInductionRotation))
  (return (.pitch _magneticinductionrotation) (.yaw _magneticinductionrotation) (* (Variables|Default|GetMagneticInductionScalar) 1e+03)))

(fn SetInductionsRotation
  (params (Alpha :type Float%20%28single-precision%29) (Beta :type Float%20%28single-precision%29) (MagneticInduction :type Float%20%28single-precision%29))
  (bind _outactors (Actor|GetAllActorsOfClass "/Game/Environment/BP_MagneticInductionVector.BP_MagneticInductionVector_C"))
  (Transformation|SetActorRotation (Utilities|Array|Get(acopy) _outactors) (Math|Rotator|MakeRotator 0.0 Alpha Beta))
  (bind _outactors_2 (Actor|GetAllActorsOfClass "/Game/Environment/BP_MagneticInductionVector_WBP.BP_MagneticInductionVector_WBP_C"))
  (Transformation|SetActorRotation (Utilities|Array|Get(acopy) _outactors_2) (Math|Rotator|MakeRotator 0.0 Alpha Beta))
  (bind _output_get (Variables|Default|SetMagneticInductionScalar (/ MagneticInduction 1e+03)))
  (bind _returnvalue (Class|CustomVectorLibrary|RadialtoVector Alpha Beta _output_get))
  (Variables|Default|SetMagneticInduction _returnvalue)
  (bind _outactors_3 (Actor|GetAllActorsOfClass "/Script/SELF.ParticalBase"))
  (for _array_element _outactors_3
    (Utilities|IsValid _array_element
      (:Is%20Valid
        (Variables|/Script/SELF.ParticalBase|SetMagneticInduction _array_element (Variables|Default|GetMagneticInduction))))))

(fn SetPause
  (params (IsPaused :type Boolean))
  (if IsPaused
    (Variables|Default|SetIsPaused true)
    (else
      (Variables|Default|SetIsPaused false)))
  (bind _outactors (Actor|GetAllActorsOfClass "/Game/Particals/BP_ParticalBase.BP_ParticalBase_C"))
  (for _array_element _outactors
    (Class|ParticalBase|SetPaused _array_element (Variables|Default|GetIsPaused))))

(fn LoopSpawnCustom
  (params (Loop :type Boolean) (Id :type Integer))
  (bind _output_get (Variables|Default|SetIsElectronLoop Loop))
  (Variables|Default|SetId Id)
  (if _output_get
    (bind _returnvalue (Utilities|Time|SetTimerbyEvent (EventDispatchers|CreateEvent :!event Custom|SpawnCustomParticle) (.Rate (Utilities|Struct|BreakParticleDataStruct (Utilities|Array|Get(acopy) (Variables|Default|GetParticle%20Data) (Variables|Default|GetId)))) true))
    (Variables|Default|SetCustomTimerHandle _returnvalue)
    (else
      (Utilities|Time|ClearandInvalidateTimerbyHandle (Variables|Default|GetCustomTimerHandle)))))