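; Axis marker actor that shows a colored arrow with a text label in the world.
; The construction script adds length and thickness variables to the arrow's relative scale and applies the arrow color.
; It also sets the label's text, size and world rotation, tinting it to match the arrow.
; The event graph holds no logic, so all setup happens at construction.
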(event EventBeginPlay)

(event Collision|EventActorBeginOverlap
  (params (OtherActor :type Actor%20Object%20Reference)))

(event EventTick
  (params (DeltaSeconds :type Float%20%28single-precision%29)))

(fn ConstructionScript
  (bind _arrow (Variables|Default|GetArrow))
  (bind _tickness (Variables|Default|GetTickness))
  (bind _axisname (Variables|Default|GetAxisName))
  (Transformation|SetRelativeScale3D _arrow (+ (Variables|/Script/Engine.SceneComponent|GetRelativeScale3D _arrow) (Math|Vector|MakeVector (Variables|Default|GetArrowLength) _tickness _tickness)))
  (Components|Arrow|SetArrowColor(LinearColor) _arrow (Variables|Default|GetArrowColor))
  (Rendering|Components|TextRender|SetText _axisname (Variables|Default|GetName))
  (Rendering|Components|TextRender|SetTextRenderColor _axisname (Math|Conversions|ToColor(LinearColor) (Variables|Default|GetArrowColor)))
  (Rendering|Components|TextRender|SetWorldSize _axisname (Variables|Default|GetTextSize))
  (Transformation|SetWorldRotation _axisname (Variables|Default|GetTextRotation) false false))